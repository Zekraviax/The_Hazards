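; Behavior tree task that picks a random patrol destination for an AI-controlled Character.
; On execute it sets the character's walk speed to PatrolSpeed, then queries a random reachable point within PatrolRadius of the pawn.
; It writes that point, or the pawn's current location if none is found, to the PatrolLocation blackboard key and finishes successfully.
; A failed Character cast exits without finishing the task.
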(event `self.ReceiveExecuteAI`
  (params (OwnerController :type "AIController Object Reference") (ControlledPawn :type "Pawn Object Reference"))
  (bind _returnvalue (`Actor.K2_GetActorLocation` ControlledPawn))
  (bind _patrollocation (`self.PatrolLocation`))
  (bind (_randomlocation _returnvalue_2) (`NavigationSystemV1.K2_GetRandomReachablePointInRadius` _returnvalue (`self.PatrolRadius`) null null))
  (bind _ascharacter (cast `Character` ControlledPawn))
  (set `CharacterMovementComponent.MaxWalkSpeed` (`self.PatrolSpeed`) (`Character.CharacterMovement` _ascharacter))
  (if _returnvalue_2
    (`BTFunctionLibrary.SetBlackboardValueAsVector` _patrollocation _randomlocation)
    (else
      (`BTFunctionLibrary.SetBlackboardValueAsVector` _patrollocation _returnvalue)))
  (`self.FinishExecute` true))