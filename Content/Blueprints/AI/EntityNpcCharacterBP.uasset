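; AI-controlled NPC character that tracks the player through AI perception.
; When it senses an EntityPlayerCharacterBp tagged "Player", it cancels the pending lose-sight timer and writes HasLineOfSight and EnemyActor to its Blackboard.
; Otherwise, an update for that class starts a one-shot timer of LineOfSightTimer length that clears both keys on expiry, giving a grace period before the NPC forgets its target.
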(event `self.AIPerception.OnTargetPerceptionUpdated`
  (params (Actor :type "Actor Object Reference") (Stimulus :type "AIStimulus Structure"))
  (bind _returnvalue (`AIBlueprintHelperLibrary.GetBlackboard` self))
  (cast `/Game/Blueprints/Player/EntityPlayerCharacterBp` Actor)
  (if (and (`self.ActorHasTag` Actor "Player") (`.bSuccessfullySensed` (break `AIStimulus` Stimulus)))
    (`KismetSystemLibrary.K2_ClearAndInvalidateTimerHandle` (`self.EnemyTimer`))
    (`BlackboardComponent.SetValueAsBool` _returnvalue "HasLineOfSight" true)
    (`BlackboardComponent.SetValueAsObject` _returnvalue "EnemyActor" Actor)
    (else
      (bind _returnvalue_2 (`KismetSystemLibrary.K2_SetTimerDelegate` (delegate `StartEnemy_Timer`) (`self.LineOfSightTimer`)))
      (set `self.EnemyTimer` _returnvalue_2))))

(event `StartEnemy_Timer`
  (bind _returnvalue (`AIBlueprintHelperLibrary.GetBlackboard` self))
  (`BlackboardComponent.SetValueAsBool` _returnvalue "HasLineOfSight" false)
  (`BlackboardComponent.SetValueAsObject` _returnvalue "EnemyActor" null))

(fn `UserConstructionScript`)