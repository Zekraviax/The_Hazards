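; Behavior tree task that picks a point for an AI pawn to flee from the enemy actor stored on the blackboard.
; It takes the look-at direction toward that actor and offsets the pawn's location a fixed distance the opposite way.
; The point keeps the pawn's current height, is written to the RunAwayLocation key without any navmesh check, and the task finishes successfully at once.
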(event `self.ReceiveExecuteAI`
  (params (OwnerController :type "AIController Object Reference") (ControlledPawn :type "Pawn Object Reference"))
  (bind _returnvalue (`Actor.K2_GetActorLocation` ControlledPawn))
  (`BTFunctionLibrary.SetBlackboardValueAsVector` (`self.RunAwayLocation`) (`KismetMathLibrary.MakeVector` (.x (+ _returnvalue (* (`KismetMathLibrary.GetForwardVector` (`KismetMathLibrary.FindLookAtRotation` _returnvalue (`Actor.K2_GetActorLocation` (`BTFunctionLibrary.GetBlackboardValueAsActor` (`self.EnemyActor`))))) -500.0))) (.y (+ _returnvalue (* (`KismetMathLibrary.GetForwardVector` (`KismetMathLibrary.FindLookAtRotation` _returnvalue (`Actor.K2_GetActorLocation` (`BTFunctionLibrary.GetBlackboardValueAsActor` (`self.EnemyActor`))))) -500.0))) (.z _returnvalue)))
  (`self.FinishExecute` true))