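; Enemy AI controller Blueprint holding a disconnected draft of behavior tree startup, so it currently runs no logic of its own.
; BeginPlay and the construction script are empty.
; The unwired chain stores the first Entity_Player_Blueprint actor in the "Enemy" blackboard key, runs Test_BehaviourTree, then prints whether the blackboard is valid.
; The blackboard write precedes the RunBehaviorTree call in that chain.
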(event `self.ReceiveBeginPlay`)

(fn `UserConstructionScript`)